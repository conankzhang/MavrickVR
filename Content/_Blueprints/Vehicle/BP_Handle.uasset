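; BP_Handle is a handle actor in the Vehicle folder that BP_MotionController can pick up and drop.
; Pickup turns off physics on the static mesh and attaches the root component to the given component, keeping the world transform.
; Drop re-enables physics and detaches the actor in place.
; Tick prints the mesh's world location every frame as debug output.
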(event EventBeginPlay)

(event Collision|EventActorBeginOverlap
  (params (OtherActor :type Actor%20Object%20Reference)))

(event EventTick
  (params (DeltaSeconds :type Float%20%28single-precision%29))
  (Development|PrintString (Utilities|String|ToString(Vector) (Transformation|GetWorldLocation (Variables|Debug|GetStaticMeshComponent)))))

(event EventPickup
  (params (AttachTo :type Scene%20Component%20Object%20Reference) (IsLeft :type Boolean))
  (Physics|SetSimulatePhysics (Variables|Debug|GetStaticMeshComponent) false)
  (Transformation|AttachComponentToComponent (VehicleSound|GetRootComponent) AttachTo "None" "KeepWorld" "KeepWorld" "KeepWorld" false))

(event EventDrop
  (params (AttachTo :type Scene%20Component%20Object%20Reference) (IsLeft :type Boolean))
  (Physics|SetSimulatePhysics (Variables|Debug|GetStaticMeshComponent) true)
  (Transformation|DetachFromActor "KeepWorld" "KeepWorld" "KeepWorld"))

(fn ConstructionScript)